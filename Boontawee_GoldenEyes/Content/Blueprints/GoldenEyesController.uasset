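; First-person shooter player Blueprint that handles movement, look with optional pitch inversion, and hitscan firing, with the gun attached to the arm mesh's hand socket.
; Fire plays an arm montage and sound, then line traces from the camera with persistent debug drawing, spawning an explosion on impact without applying damage.
; It creates the FPS HUD widget and updates HP percentage each Tick; right mouse subtracts HP directly, while point-damage handling is empty.
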(event EventBeginPlay
  (bind _returnvalue (UserInterface|CreateWidget "/Game/UIAssets/FPS_UI.FPS_UI_C"))
  (UserInterface|Viewport|AddtoViewport _returnvalue 0))

(event Collision|EventActorBeginOverlap
  (params (OtherActor :type Actor%20Object%20Reference)))

(event EventTick
  (params (DeltaSeconds :type Float%20%28single-precision%29))
  ;[1 1 1] Update HP
  (Variables|Default|SetHPPercentage (/ (Variables|Default|GetHP) (Variables|Default|GetMaxHP))))

(event Game|Damage|EventPointDamage
  (params (Damage :type Float%20%28single-precision%29) (DamageType :type Damage%20Type%20Object%20Reference) (HitLocation :type Vector :default "0, 0, 0") (HitNormal :type Vector :default "0, 0, 0") (HitComponent :type Primitive%20Component%20Object%20Reference) (BoneName :type Name :default "None") (ShotFromDirection :type Vector :default "0, 0, 0") (InstigatedBy :type Controller%20Object%20Reference) (DamageCauser :type Actor%20Object%20Reference) (HitInfo :type Hit%20Result%20Structure%20%28by%20ref%29)))

(event Input|ActionEvents|InputActionFire
  (params (Key :type Key%20Structure :default "None"))
  (bind _fpscamera (Variables|Default|GetFPSCamera))
  (bind _returnvalue (Transformation|GetWorldLocation _fpscamera))
  (:Pressed
    (Animation|Montage|PlayMontage (Variables|Default|GetFPSArm) "/Game/Models/Animations/Shoot_MT.Shoot_MT"
      (:then
        (Audio|PlaySoundatLocation "/Game/StarterContent/Audio/Explosion_Cue.Explosion_Cue" (Transformation|GetWorldLocation (Variables|Default|GetFPSCamera)) "0, 0, 0" 1.0 1.0 0.0 0 0 0)
        (bind (_outhit _returnvalue_2) (Collision|LineTraceByChannel _returnvalue (+ _returnvalue (* (Math|Vector|GetForwardVector (Transformation|GetWorldRotation _fpscamera)) (Variables|Default|GetGunRange))) "TraceTypeQuery2" false 0 "Persistent"))
        (if _returnvalue_2
          (Effects|SpawnEmitteratLocation "/Game/StarterContent/Particles/P_Explosion.P_Explosion" (.ImpactPoint (Collision|BreakHitResult _outhit)) "0, 0, 0" "0.500000,0.500000,0.500000"))))))

(event Input|AxisEvents|InputAxisMoveForward
  (params (AxisValue :type Float%20%28single-precision%29))
  ;[1 1 1] Locomotion Movement
  (Pawn|Input|AddMovementInput (Transformation|GetActorForwardVector) AxisValue false))

(event Input|AxisEvents|InputAxisMoveRight
  (params (AxisValue :type Float%20%28single-precision%29))
  ;[1 1 1] Locomotion Movement
  (Pawn|Input|AddMovementInput (Transformation|GetActorRightVector) AxisValue false))

(event Input|AxisEvents|InputAxisLookUp
  (params (AxisValue :type Float%20%28single-precision%29))
  ;[1 1 1] Locomotion Movement
  (if (Variables|Default|GetInvertLook)
    (Pawn|Input|AddControllerPitchInput AxisValue)
    (else
      (Pawn|Input|AddControllerPitchInput (* AxisValue -1.0)))))

(event Input|AxisEvents|InputAxisTurn
  (params (AxisValue :type Float%20%28single-precision%29))
  ;[1 1 1] Locomotion Movement
  (Pawn|Input|AddControllerYawInput AxisValue))

(event Input|MouseEvents|RightMouseButton
  (params (Key :type Key%20Structure :default "None"))
  (:Pressed
    ;[1 1 1] Take Damage
    (Variables|Default|SetHP (- (Variables|Default|GetHP) 1e+01))))

(fn ConstructionScript
  (Transformation|AttachComponentToComponent (Variables|Default|GetGun) (Variables|Default|GetFPSArm) "RightHandSocket" "KeepRelative" "KeepRelative" "KeepRelative" true))